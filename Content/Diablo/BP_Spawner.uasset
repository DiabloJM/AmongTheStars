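; Enemy spawner actor that spawns a limited number of CubeEnemy actors during play.
; On BeginPlay a looping timer fires the spawn event every few seconds.
; Each tick of the timer places an enemy at the transform of a random actor from SpawnLocations until the spawn counter reaches its cap.
; The counter only increments, so the cap limits total spawns rather than living enemies.
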(event Custom|Spawn%20Enemy
  (if (< (Variables|Default|GetEnemiesSpawned) 5)
    (bind _result (Math|Integer|IncrementInt (Variables|Default|GetEnemiesSpawned))
      (:%20%20
        (Variables|Default|SetEnemiesSpawned _result)
        (Game|SpawnActorfromClass "/Game/Diablo/CubeEnemy.CubeEnemy_C" (Transformation|GetActorTransform (.OutItem (Utilities|Array|Random (Variables|Default|GetSpawnLocations)))) "Undefined" 0 0)))))

(event EventBeginPlay
  (Utilities|Time|SetTimerbyEvent (delegate Custom|Spawn%20Enemy) 3.0 true))

(fn ConstructionScript)